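; AC_Interaction is an actor component that lets its owner look at and interact with actors implementing BPI_Interact.
; Each tick it line-traces on Visibility from the owner's eye viewpoint up to InteractRange, setting or clearing CurrentInteractable.
; A W_Interaction widget, created on BeginPlay, shows the target's interaction message.
; The IA_Interact input sends InteractMessage to the current target, passing the owning C_Player.
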(event Input|EnhancedActionEvents|EnhancedInputActionIA_Interact
  (params (ActionValue :type Boolean) (ElapsedSeconds :type Float%20%28double-precision%29) (TriggeredSeconds :type Float%20%28double-precision%29) (InputAction :type Input%20Action%20Object%20Reference :default "/Game/Blueprints/Framework/Input/IA_Interact.IA_Interact"))
  (bind _currentinteractable (Variables|Private|GetCurrentInteractable)
    (:then
      (Class|BPIInteract|Interact(Message) _currentinteractable (.AsC%20Player (Utilities|Casting|CastToC_Player (Components|GetOwner)))))
    (:else)))

(fn ReceiveTick
  (params (DeltaSeconds :type Float%20%28single-precision%29))
  (bind _hitactor (Utilities|TracefromOwnerEyes)
    (:Hit
      (if (!= (Variables|Private|GetCurrentInteractable) _hitactor)
        (if (Utilities|DoesObjectImplementInterface _hitactor "/Game/Blueprints/Interfaces/BPI_Interact.BPI_Interact_C")
          (Private|SetInteractable _hitactor)
          (else
            (Private|ClearInteractable)))))
    (:NoHit
      (Private|ClearInteractable))))

(fn SetInteractable
  (params (NewInteractable :type Object%20Object%20Reference))
  (bind _output_get (Variables|Private|SetCurrentInteractable NewInteractable))
  (bind _message (Class|BPIInteract|GetInteractMessage(Message) _output_get))
  (Rendering|Components|TextRender|SetText (Variables|/Game/Blueprints/Widget/W_Interaction.W_Interaction_C|GetInteractionText (Variables|Private|GetInteractWidget)) _message))

(fn ClearInteractable
  (Variables|Private|GetCurrentInteractable
    (:then
      (Variables|Private|SetCurrentInteractable 0)
      (Rendering|Components|TextRender|SetText (Variables|/Game/Blueprints/Widget/W_Interaction.W_Interaction_C|GetInteractionText (Variables|Private|GetInteractWidget)) ""))
    (:else)))

(fn ReceiveBeginPlay
  (bind _returnvalue (UserInterface|CreateWidget "/Game/Blueprints/Widget/W_Interaction.W_Interaction_C"))
  (bind _output_get (Variables|Private|SetInteractWidget _returnvalue))
  (UserInterface|Viewport|AddtoViewport _output_get 0))